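; BP_Crusher is an obstacle that moves a crusher cube up and down and sends the player back to a restart point on contact.
; On BeginPlay it starts the looping CrusherMovement timeline, whose CrusherHeight track sets the cube's relative Z.
; Box overlaps cast the other actor to BP_Player and teleport it to the transform of RestartTransformTarget.
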(event OnComponentBeginOverlap(Box)
  (params (OverlappedComponent :type Primitive%20Component%20Object%20Reference) (OtherActor :type Actor%20Object%20Reference) (OtherComp :type Primitive%20Component%20Object%20Reference) (OtherBodyIndex :type Integer) (bFromSweep :type Boolean) (SweepResult :type Hit%20Result%20Structure%20%28by%20ref%29))
  (bind _asbp_player (Utilities|Casting|CastToBP_Player OtherActor))
  (Transformation|SetActorTransform _asbp_player (Transformation|GetActorTransform (Variables|Default|GetRestartTransformTarget)) false true))

(event EventBeginPlay
  (Components|Timeline|SetLooping (Variables|Default|GetCrusherMovement) true)
  (Components|Timeline|PlayfromStart (Variables|Default|GetCrusherMovement)))

(fn ConstructionScript)