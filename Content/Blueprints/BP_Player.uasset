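; Player pawn with timeline-driven forward/backward movement, turning and a switchable Levitation or Time Slowdown ability.
; Releasing movement keys lets the looping Movement timeline finish its cycle; turns cannot start while moving, or movement while turning.
; Ability and cooldown timelines gate reuse and feed the HUD progress bar.
; Tick applies manual falling, suspended by trace-based levitation; slowdown offsets global dilation with the pawn's CustomTimeDilation to keep player speed.
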(event EventBeginPlay
  (Components|Movement|SetUpdatedComponent (Variables|Default|GetFloatingPawnMovement) (Variables|Default|GetSphere))
  (Components|Timeline|SetPlayRate (Variables|Default|GetMovement) (/ 1.0 (Variables|Default|GetMovementTimeMultiplier)))
  (CallFunction|SetupUI))

(event EventTick
  (params (DeltaSeconds :type Float%20%28single-precision%29))
  (Movement|Fall DeltaSeconds))

(event Input|KeyboardEvents|W
  (params (Key :type Key%20Structure :default "None"))
  (:Pressed
    (if (not (Movement|IsRotating))
      (Movement|StartMovingForward)))
  (:Released
    (Movement|StopMovingForward)))

(event Input|KeyboardEvents|S
  (params (Key :type Key%20Structure :default "None"))
  (:Pressed
    (if (not (Movement|IsRotating))
      (Movement|StartMovingBackward)))
  (:Released
    (Movement|StopMovingBackward)))

(event Input|KeyboardEvents|A
  (params (Key :type Key%20Structure :default "None"))
  (:Pressed
    (if (not (or (Movement|IsRotating) (Movement|IsMoving)))
      (Movement|StartRotation "NewEnumerator0"))))

(event Input|KeyboardEvents|D
  (params (Key :type Key%20Structure :default "None"))
  (:Pressed
    (if (not (or (Movement|IsRotating) (Movement|IsMoving)))
      (Movement|StartRotation "NewEnumerator1"))))

(event Input|KeyboardEvents|Escape
  (params (Key :type Key%20Structure :default "None"))
  (:Pressed
    (Game|QuitGame 0 "Quit" false)))

(event Input|KeyboardEvents|E
  (params (Key :type Key%20Structure :default "None"))
  (:Pressed
    (Ability|ExecuteAbiliity)))

(fn ConstructionScript)

(fn StartMovingForward
  (if (Class|TimelineComponent|IsReversing (Variables|Default|GetMovement))
    (Audio|Components|Audio|Stop (Variables|Default|GetMovement))
    (Components|Timeline|SetLooping (Variables|Default|GetMovement) false)
    (else
      (if (Audio|Components|Audio|IsPlaying (Variables|Default|GetMovement))
        _
        (else
          (Components|Timeline|PlayfromStart (Variables|Default|GetMovement))))
      (Components|Timeline|SetLooping (Variables|Default|GetMovement) true))))

(fn StopMovingForward
  (bind _movement (Variables|Default|GetMovement))
  (if (and (Audio|Components|Audio|IsPlaying _movement) (not (Class|TimelineComponent|IsReversing _movement)))
    (Components|Timeline|SetLooping (Variables|Default|GetMovement) false)))

(fn StartMovingBackward
  (bind _movement (Variables|Default|GetMovement))
  (if (and (Audio|Components|Audio|IsPlaying _movement) (not (Class|TimelineComponent|IsReversing _movement)))
    (Audio|Components|Audio|Stop (Variables|Default|GetMovement))
    (Components|Timeline|SetLooping (Variables|Default|GetMovement) false)
    (else
      (if (Class|TimelineComponent|IsReversing (Variables|Default|GetMovement))
        _
        (else
          (Components|Timeline|ReversefromEnd (Variables|Default|GetMovement))))
      (Components|Timeline|SetLooping (Variables|Default|GetMovement) true))))

(fn StopMovingBackward
  (if (Class|TimelineComponent|IsReversing (Variables|Default|GetMovement))
    (Components|Timeline|SetLooping (Variables|Default|GetMovement) false)))

(fn IsRotating
  (return (!= 0.0 (Variables|Default|GetRotationMultiplier))))

(fn IsMoving
  (return (Audio|Components|Audio|IsPlaying (Variables|Default|GetMovement))))

(fn StartRotation
  (params (Direction :type E_RotationDirection%20Enum :default "NewEnumerator0"))
  (Variables|Default|SetStartYaw (.yaw (Transformation|GetActorRotation)))
  (Variables|Default|SetRotationMultiplier (Utilities|Select :Index Direction :NewEnumerator0 -1.0 :NewEnumerator1 1.0))
  (Components|Timeline|PlayfromStart (Variables|Default|GetRotation)))

(fn Fall
  (params (DeltaTime :type Float%20%28double-precision%29))
  (if (Variables|Default|GetbFallingEnabled)
    (Pawn|Input|AddMovementInput "0.000000,0.000000,-1.000000" (* DeltaTime 5e+01) false)))

(fn StartLevitating
  (bind (_start _end) (|GetLineTraceLocations))
  (bind _returnvalue (Collision|LineTraceByChannel _start _end "TraceTypeQuery1" false 0 "None"))
  (Variables|Default|SetbFallingEnabled (not _returnvalue))
  (if _returnvalue
    (Pawn|Input|AddMovementInput "0.000000,0.000000,1.000000" 1.0 false)))

(fn StopLevitating
  (Variables|Default|SetbFallingEnabled true))

(fn StartTimeSlowdown
  (Utilities|Time|SetGlobalTimeDilation 0.25)
  (Variables|Default|SetCustomTimeDilation 4.0))

(fn StopTimeSlowdown
  (Utilities|Time|SetGlobalTimeDilation 1.0)
  (Variables|Default|SetCustomTimeDilation 1.0))

(fn ExecuteAbiliity
  (if (not (or (Ability|IsAbililityRecharging) (Ability|IsAbililityWorking)))
    (Components|Timeline|PlayfromStart (Variables|Default|GetAbility))))

(fn SetupUI
  (bind _returnvalue (UserInterface|CreateWidget "/Game/Blueprints/W_HUD.W_HUD_C"))
  (bind _output_get (Variables|Default|SetHUD _returnvalue))
  (UserInterface|Viewport|AddtoViewport _output_get 0))

(fn IsAbililityRecharging
  (return (Audio|Components|Audio|IsPlaying (Variables|Default|GetAbilityCooldown))))

(fn IsAbililityWorking
  (return (Audio|Components|Audio|IsPlaying (Variables|Default|GetAbility))))

(fn SetSelectedAbility
  (params (NewAbility :type E_AbilityType%20Enum :default "NewEnumerator0"))
  (Audio|Components|Audio|Stop (Variables|Default|GetAbility))
  (Components|Timeline|PlayfromStart (Variables|Default|GetAbilityCooldown))
  (bind _output_get (Variables|Default|SetSelectedAbility NewAbility))
  (Default|SetAbilityName (Variables|Default|GetHUD) _output_get))